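; BP_StateRunnerGameMode is the game mode that manages the gameplay HUD and the game-over screen.
; On BeginPlay it adds WBP_GameHUD to the viewport, exposes it through GetGameHUDWidget and binds to the lives component's player-died event.
; On death it shows WBP_GameOver with UI-only input and the cursor hidden.
; Short delays let that widget take keyboard focus before the game pauses.
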(event Custom|OnPlayerDeath
  (bind _returnvalue (Game|GetPlayerController 0))
  (bind _returnvalue_2 (UserInterface|CreateWidget "/Game/_DEVELOPER/UI/WBP_GameOver.WBP_GameOver_C" (Game|GetPlayerController 0)))
  (bind _output_get (Variables|Default|SetGameOverInstance _returnvalue_2))
  (UserInterface|Viewport|AddtoViewport _output_get 0)
  (Variables|/Script/Engine.PlayerController|SetbShowMouseCursor _returnvalue false)
  (Input|SetInputModeUIOnly _returnvalue (Variables|Default|GetGameOverInstance) "DoNotLock" false)
  (Utilities|FlowControl|Delay 0.1)
  (Class|ArcadeMenuWidget|TakeKeyboardFocus (Variables|Default|GetGameOverInstance))
  (Utilities|FlowControl|Delay 0.2)
  (Game|SetGamePaused true))

(event EventBeginPlay
  (|CallParentFunction)
  (bind _returnvalue (UserInterface|CreateWidget "/Game/_DEVELOPER/UI/WBP_GameHUD.WBP_GameHUD_C" (Game|GetPlayerController 0)))
  (bind _output_get (Variables|Default|SetGameHUDInstance _returnvalue))
  (UserInterface|Viewport|AddtoViewport _output_get 0)
  (EventDispatchers|BindEventtoOnPlayerDied (Variables|Default|GetLivesSystemComponent) (delegate Custom|OnPlayerDeath)))

(event EventTick
  (params (DeltaSeconds :type Float%20%28single-precision%29)))

(fn ConstructionScript)

(fn GetGameHUDWidget
  (return (Variables|Default|GetGameHUDInstance)))