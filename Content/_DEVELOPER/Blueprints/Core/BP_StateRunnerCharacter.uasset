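; Player character Blueprint for StateRunner Arcade that adds the input mapping context and drives power-up and damage visuals.
; Tick eases the mesh into a roll while Overclock is active, and game mode component events toggle Overclock VFX.
; DamageListener binds itself to damage events and blinks the mesh via a looping timer, so the flash also runs on BeginPlay.
; OnMagnetEffectChanged toggles two magnet effects, with no binding in this graph.
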(event Custom|FlashTick
  ;[0.15 0.15 0.15 0.5] Damage Flash VFX for Character Mesh
  ;;[0.15 0.15 0.15 0.5] Function used in timer
  (Rendering|ToggleVisibility (Variables|Character|GetMesh) false))

(event Custom|OnOverclockChanged
  (params (bIsActive :type Boolean))
  (bind _overclockvfx (Variables|Default|GetOverclockVFX))
  ;[0.15 0.15 0.15 0.5] Overclock VFX
  (if bIsActive
    (Components|Activation|SetActive _overclockvfx true false)
    (else
      (Components|Activation|SetActive _overclockvfx false false))))

(event Custom|PlayerControlsListener
  ;[0.15 0.15 0.15 0.5] Player Controls
  (bind _asplayer_controller (Utilities|Casting|CastToPlayerController (Pawn|GetController)))
  (Input|AddMappingContext (PlayerController|LocalPlayerSubsystems|GetEnhancedInputLocalPlayerSubsystem _asplayer_controller) "/Game/Input/IMC_Default.IMC_Default" 0 "(bIgnoreAllPressedKeysUntilRelease=True,bForceImmediately=False,bNotifyUserSettings=False)"))

(event Custom|OverclockListener
  ;[0.15 0.15 0.15 0.5] Overclock VFX
  (bind _asstate_runner_arcade_game_mode (Utilities|Casting|CastToStateRunner_ArcadeGameMode (Game|GetGameMode)))
  (EventDispatchers|BindEventtoOnOverclockStateChanged (Class|StateRunnerArcadeGameMode|GetOverclockSystemComponent _asstate_runner_arcade_game_mode) (delegate Custom|OnOverclockChanged)))

(event Custom|DamageListener
  (params (RemainingLives :type Integer))
  ;[0.15 0.15 0.15 0.5] Damage Flash VFX for Character Mesh
  (bind _asstate_runner_arcade_game_mode (Utilities|Casting|CastToStateRunner_ArcadeGameMode (Game|GetGameMode)))
  (EventDispatchers|BindEventtoOnDamageTaken (Variables|/Script/StateRunner_Arcade.StateRunner_ArcadeGameMode|GetLivesSystemComponent _asstate_runner_arcade_game_mode) (delegate Custom|DamageListener))
  (bind _returnvalue (Utilities|Time|SetTimerbyFunctionName 0 "FlashTick" 0.075 true))
  (bind _output_get (Variables|Default|SetDamageTakenHandle _returnvalue))
  (Utilities|FlowControl|Delay 0.7)
  (Utilities|Time|ClearandInvalidateTimerbyHandle _output_get)
  (Rendering|SetVisibility (Variables|Character|GetMesh) true false))

(event EventBeginPlay
  ;[0.15 0.15 0.15 0.5] Setting up listeners--all hapens before first frame
  (Utilities|FlowControl|Sequence
    (:then_0
      (CallFunction|PlayerControlsListener))
    (:then_1
      (CallFunction|OverclockListener))
    (:then_2
      (CallFunction|DamageListener))))

(event EventTick
  (params (DeltaSeconds :type Float%20%28single-precision%29))
  (bind _asstate_runner_arcade_game_mode (Utilities|Casting|CastToStateRunner_ArcadeGameMode (Game|GetGameMode)))
  (Transformation|SetRelativeRotation (Variables|Character|GetMesh) (Math|Interpolation|RInterpTo (Variables|/Script/Engine.SceneComponent|GetRelativeRotation (Variables|Character|GetMesh)) (select (Variables|/Script/StateRunner_Arcade.OverclockSystemComponent|GetbIsOverclockActive (Variables|/Script/StateRunner_Arcade.StateRunner_ArcadeGameMode|GetOverclockSystemComponent _asstate_runner_arcade_game_mode)) (Math|Rotator|MakeRotator 2e+01 0.0 -9e+01) (Math|Rotator|MakeRotator 0.0 0.0 -9e+01)) DeltaSeconds 5.0) false false))

(event EventOnMagnetEffectChanged
  (params (bIsActive :type Boolean))
  (bind _magnetvfx (Variables|Default|GetMagnetVFX))
  (bind _magnetvfx2_ring (Variables|Default|GetMagnetVFX2_RING))
  (if bIsActive
    (Components|Activation|Activate _magnetvfx false)
    (Components|Activation|Activate _magnetvfx2_ring false)
    (else
      (Components|Activation|Deactivate _magnetvfx)
      (Components|Activation|Deactivate _magnetvfx2_ring))))

(fn ConstructionScript)