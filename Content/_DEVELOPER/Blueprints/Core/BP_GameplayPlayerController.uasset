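; BP_GameplayPlayerController is the gameplay player controller, handling the match-start input lock and the pause menu.
; BeginPlay disables input for a five-second countdown, then restores it in game-only mode with the cursor hidden.
; IA_Pause creates WBP_PauseMenu with UI-only input and delayed keyboard focus, or just restores game-only input if the menu exists.
; The menu's close event clears the stored widget reference.
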(event Custom|OnPauseMenuClosedHandler
  ;[0.15 0.15 0.15 0.5] If Pause hasnt been pressed and is pressed, creates widget and adds to viewport
  (Variables|Default|SetPauseMenuInstance 0))

(event Input|EnhancedActionEvents|EnhancedInputActionIA_Pause
  (params (ActionValue :type Boolean) (ElapsedSeconds :type Float%20%28double-precision%29) (TriggeredSeconds :type Float%20%28double-precision%29) (InputAction :type Input%20Action%20Object%20Reference :default "/Game/Input/Actions/IA_Pause.IA_Pause"))
  (if (Utilities|IsValid (Variables|Default|GetPauseMenuInstance))
    ;[0.15 0.15 0.15 0.5] Resume if Pause already pressed
    (Input|SetInputModeGameOnly (Game|GetPlayerController 0) false)
    (Variables|Default|SetbShowMouseCursor false)
    (else
      ;[0.15 0.15 0.15 0.5] If Pause hasnt been pressed and is pressed, creates widget and adds to viewport
      (bind _returnvalue (UserInterface|CreateWidget "/Game/_DEVELOPER/UI/WBP_PauseMenu.WBP_PauseMenu_C"))
      (bind _output_get (Variables|Default|SetPauseMenuInstance _returnvalue))
      (EventDispatchers|BindEventtoOnPauseMenuClosed _output_get (delegate Custom|OnPauseMenuClosedHandler))
      (UserInterface|Viewport|AddtoViewport _output_get 0)
      (Variables|Default|SetbShowMouseCursor self false)
      (Input|SetInputModeUIOnly (Game|GetPlayerController 0) (Variables|Default|GetPauseMenuInstance) "DoNotLock" false)
      (Utilities|FlowControl|Delay 0.1)
      (Class|ArcadeMenuWidget|TakeKeyboardFocus (Variables|Default|GetPauseMenuInstance)))))

(event EventBeginPlay
  ;[0.15 0.15 0.15 0.5] Delay for Countdown before player controls available
  (Input|DisableInput (Game|GetPlayerController 0))
  (Utilities|FlowControl|Delay 5.0)
  (Input|EnableInput (Game|GetPlayerController 0))
  (Input|SetInputModeGameOnly self false)
  (Variables|Default|SetbShowMouseCursor false))

(event EventTick
  (params (DeltaSeconds :type Float%20%28single-precision%29)))

(fn ConstructionScript)