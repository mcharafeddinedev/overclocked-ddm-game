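; Player controller for the main menu that creates and shows the main menu widget on BeginPlay.
; After short delays it switches to UI-only input, hides the mouse cursor and gives the widget user focus.
; It then prints whether the widget has keyboard focus as a debug check.
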(event EventBeginPlay
  (bind _returnvalue (UserInterface|CreateWidget "/Game/_DEVELOPER/UI/MainMenu/WBP_MainMenu.WBP_MainMenu_C" (Game|GetPlayerController 0)))
  (bind _output_get (Variables|Default|SetMainMenuWidget _returnvalue))
  (UserInterface|Viewport|AddtoViewport _output_get 0)
  (Utilities|FlowControl|Delay 0.1)
  (Input|SetInputModeUIOnly self (Variables|Default|GetMainMenuWidget) "DoNotLock" false)
  (Variables|Default|SetbShowMouseCursor false)
  (Utilities|FlowControl|Delay 0.2)
  (Class|Widget|SetUserFocus (Variables|Default|GetMainMenuWidget) self)
  (Development|PrintString (Utilities|String|Append "Keyboard Focus:" (Utilities|String|ToString(Boolean) (Class|Widget|HasKeyboardFocus (Variables|Default|GetMainMenuWidget))))))

(event EventTick
  (params (DeltaSeconds :type Float%20%28single-precision%29)))

(fn ConstructionScript)