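; BP_TrackSegment is a track piece that scrolls along negative X in the State Runner game mode.
; On BeginPlay it caches the game mode's world scroll component.
; While scrolling is enabled, Tick moves it by that component's current speed times delta time, rounding X to a whole number each frame.
; Once X drops below the despawn threshold, the segment destroys itself and prints a debug message.
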(event EventBeginPlay
  (bind _asbp_state_runner_game_mode (Utilities|Casting|CastToBP_StateRunnerGameMode (Game|GetGameMode)))
  (Variables|Default|SetScroll%20Component (Class|StateRunnerArcadeGameMode|GetWorldScrollComponent _asbp_state_runner_game_mode)))

(event EventTick
  (params (DeltaSeconds :type Float%20%28single-precision%29))
  (bind _returnvalue (Transformation|GetActorLocation))
  (bind _scroll_component (Variables|Default|GetScroll%20Component))
  (if (Utilities|IsValid _scroll_component)
    (if (Class|WorldScrollComponent|IsScrollingEnabled _scroll_component)
      (Transformation|SetActorLocation (Math|Vector|MakeVector (Math|Conversions|ToFloat(Integer) (Math|Float|Round (- (.x _returnvalue) (* (Variables|/Script/StateRunner_Arcade.WorldScrollComponent|GetCurrentScrollSpeed _scroll_component) DeltaSeconds)))) (.y _returnvalue) (.z _returnvalue)) false false)
      ;[0.15 0.15 0.15 0.5] Check Segment against Despawn Threshold X to order destruction/garbage collection
      (if (< (.x (Transformation|GetActorLocation)) (Variables|Default|GetDespawnThresholdX))
        (Actor|DestroyActor)
        (Development|PrintString "Track Segment Destroyed (Garbage Collection in BP_TrackSegment EventTick)" true true "(R=1.000000,G=0.000000,B=0.774820,A=1.000000)")))))

(fn ConstructionScript)